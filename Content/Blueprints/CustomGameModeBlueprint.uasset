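; Game mode Blueprint that tracks the player's score and handles progression through a fixed number of levels.
; On BeginPlay it sets the level count and name prefix, then restores the score from CustomGameInstance, which carries it between level loads.
; An addScore event increments the score.
; On levelComplete it saves the score to the game instance and opens the next numbered level, or GameOver after the last.
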(event Custom|addScore
  (params (incrementScore :type Integer))
  ;[1 1 1] function for incrementing score
  (Variables|Default|SetuserScore (+ (Variables|Default|GetuserScore) incrementScore)))

(event Custom|levelComplete
  ;[1 1 1] store users current store in game instance
  (bind _ascustom_game_instance (Utilities|Casting|CastToCustomGameInstance (Game|GetGameInstance)))
  (Variables|/Game/Blueprints/CustomGameInstance.CustomGameInstance_C|SetusersFullScore _ascustom_game_instance (Variables|Default|GetuserScore))
  ;[1 1 1] check if last level
  (if (< (Variables|Default|GetcurrLevel) (Variables|Default|GetLEVELAMOUNT))
    ;[1 1 1] load next level
    (Game|OpenLevel(byName) (Utilities|String|StringToName (Utilities|String|Append (Variables|Default|GetLEVELNAME) (Utilities|String|ToString(Integer) (+ (Variables|Default|GetcurrLevel) 1)))))
    (else
      ;[1 1 1] Game Over
      (Game|OpenLevel(byName) "GameOver"))))

(event EventBeginPlay
  ;[1 1 1] variable initliasation
  (Variables|Default|SetLEVELAMOUNT 3)
  (Variables|Default|SetLEVELNAME "Level")
  (bind _ascustom_game_instance (Utilities|Casting|CastToCustomGameInstance (Game|GetGameInstance)))
  (Variables|Default|SetuserScore (Variables|/Game/Blueprints/CustomGameInstance.CustomGameInstance_C|GetusersFullScore _ascustom_game_instance)))

(fn ConstructionScript)