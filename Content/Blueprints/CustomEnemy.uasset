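; CustomEnemy is a sprite-based enemy that patrols side to side and kills the player on contact.
; Tick sweeps the actor one unit along X each frame and flips its direction when the move fails, with no delta-time scaling.
; A hit on the sprite by the player character calls Death on CharacterBlueprint, guarded by a flag so it fires only once.
; The overlap event is an empty stub.
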(event OnComponentHit(PaperSprite)
  (params (HitComponent :type Primitive%20Component%20Object%20Reference) (OtherActor :type Actor%20Object%20Reference) (OtherComp :type Primitive%20Component%20Object%20Reference) (NormalImpulse :type Vector :default "0, 0, 0") (Hit :type Hit%20Result%20Structure%20%28by%20ref%29))
  ;[1 1 1] Collision with player logic
  (if (== (Game|GetPlayerCharacter 0) OtherActor)
    (if (Variables|Default|Getuntouched)
      (Variables|Default|Setuntouched false)
      (bind _ascharacter_blueprint (Utilities|Casting|CastToCharacterBlueprint (Game|GetPlayerCharacter 0)))
      (Default|Death _ascharacter_blueprint))))

(event EventBeginPlay
  ;[1 1 1] init
  (Variables|Default|SetmovingDir 1)
  (Variables|Default|Setuntouched true))

(event Collision|EventActorBeginOverlap
  (params (OtherActor :type Actor%20Object%20Reference))
  ;[1 1 1] alternative solutions for when collision is funny
)

(event EventTick
  (params (DeltaSeconds :type Float%20%28single-precision%29))
  ;[1 1 1] keep character moving side to side
  (bind _returnvalue (Transformation|SetActorLocation (+ (Transformation|GetActorLocation) (Math|Vector|MakeVector (Math|Conversions|ToFloat(Integer) (Variables|Default|GetmovingDir)) 0.0 0.0)) true false))
  (if (not _returnvalue)
    (Variables|Default|SetmovingDir (* (Variables|Default|GetmovingDir) -1))))

(fn ConstructionScript)